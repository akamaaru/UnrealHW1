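; Procedural dungeon generator that builds a run of rooms from a starting room to an end room.
; On BeginPlay it spawns the first room, adjusts its walls and places a random door at each exit, storing that exit on the door.
; SpawnNextRoom, not called here, adds a random room at SelectedExit with new doors.
; Once RoomAmount runs out, it spawns BP_EndRoom there instead, without doors.
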(event Custom|Spawn%20Doors
  ;[1 0.6156 0.3701] Spawn Doors
  (for _array_element (Variables|Default|GetExitsList)
    (bind _returnvalue (Game|SpawnActorfromClass (.OutItem (Utilities|Array|Random (Variables|Default|GetDoorTypes))) (Transformation|GetWorldTransform _array_element) "AlwaysSpawn" "MultiplyWithRoot" 0 0))
    (bind _asbp_door (Utilities|Casting|CastToBP_Door _returnvalue))
    (Variables|/Game/ProceduralDungeon/BP_Door.BP_Door_C|SetExitReference _asbp_door _array_element)))

(event Custom|Spawn%20Initial%20Room
  ;[0.0452 0.4323 0] Spawn Initial Room
  (bind _returnvalue (Game|SpawnActorfromClass "/Game/ProceduralDungeon/BP_DungeonRoom3.BP_DungeonRoom3_C" (Transformation|GetWorldTransform (Variables|Default|GetDefaultSceneRoot)) "AlwaysSpawn" "MultiplyWithRoot" 0 0))
  (Rendering|SetVisibility (Variables|/Game/ProceduralDungeon/BP_MasterRoom.BP_MasterRoom_C|GetWall2 _returnvalue) false false)
  (Transformation|SetWorldTransform (Variables|/Game/ProceduralDungeon/BP_MasterRoom.BP_MasterRoom_C|GetWall3 _returnvalue) (Math|Transform|MakeTransform (Math|Vector|MakeVector (.x (.location (Transformation|GetWorldTransform (Variables|/Game/ProceduralDungeon/BP_MasterRoom.BP_MasterRoom_C|GetWall3 _returnvalue)))) 0.0 (.z (.location (Transformation|GetWorldTransform (Variables|/Game/ProceduralDungeon/BP_MasterRoom.BP_MasterRoom_C|GetWall3 _returnvalue))))) (.rotation (Transformation|GetWorldTransform (Variables|/Game/ProceduralDungeon/BP_MasterRoom.BP_MasterRoom_C|GetWall3 _returnvalue))) (Math|Vector|MakeVector (.x (.scale (Transformation|GetWorldTransform (Variables|/Game/ProceduralDungeon/BP_MasterRoom.BP_MasterRoom_C|GetWall3 _returnvalue)))) 2e+01 (.z (.scale (Transformation|GetWorldTransform (Variables|/Game/ProceduralDungeon/BP_MasterRoom.BP_MasterRoom_C|GetWall3 _returnvalue)))))) false false)
  (bind _output_get (Variables|Default|SetCurrentRoom _returnvalue))
  (Variables|Default|SetLastRoom _output_get)
  (Utilities|Array|AppendArray (Variables|Default|GetExitsList) (Components|GetChildrenComponents (Variables|/Game/ProceduralDungeon/BP_MasterRoom.BP_MasterRoom_C|GetExits%20Folder (Variables|Default|GetCurrentRoom)) false))
  (CallFunction|SpawnDoors))

(event Custom|Spawn%20Next%20Room
  ;[0.5948 1 0.3391] Spawn Next Room
  (if (> (Variables|Default|GetRoomAmount) 0)
    (Variables|Default|SetRoomAmount (- (Variables|Default|GetRoomAmount) 1))
    (Utilities|Array|Clear (Variables|Default|GetExitsList))
    (bind _returnvalue (Game|SpawnActorfromClass (.OutItem (Utilities|Array|Random (Variables|Default|GetRoomTypes))) (Transformation|GetWorldTransform (Variables|Default|GetSelectedExit)) "AlwaysSpawn" "MultiplyWithRoot" 0 0))
    (Variables|Default|SetLastRoom (Variables|Default|GetCurrentRoom))
    (bind _asbp_master_room (Utilities|Casting|CastToBP_MasterRoom _returnvalue))
    (Variables|Default|SetCurrentRoom _asbp_master_room)
    (Utilities|Array|AppendArray (Variables|Default|GetExitsList) (Components|GetChildrenComponents (Variables|/Game/ProceduralDungeon/BP_MasterRoom.BP_MasterRoom_C|GetExits%20Folder (Variables|Default|GetCurrentRoom)) false))
    (CallFunction|SpawnDoors)
    (else
      (CallFunction|SpawnFinalRoom))))

(event Custom|Spawn%20Final%20Room
  ;[1 0.9399 0.1794] Spawn Final Room
  (bind _returnvalue (Game|SpawnActorfromClass "/Game/ProceduralDungeon/BP_EndRoom.BP_EndRoom_C" (Transformation|GetWorldTransform (Variables|Default|GetSelectedExit)) "AlwaysSpawn" "MultiplyWithRoot" 0 0))
  (Variables|Default|SetLastRoom (Variables|Default|GetCurrentRoom))
  (bind _asbp_master_room (Utilities|Casting|CastToBP_MasterRoom _returnvalue))
  (Variables|Default|SetCurrentRoom _asbp_master_room))

(event EventBeginPlay
  (CallFunction|SpawnInitialRoom))

(event Collision|EventActorBeginOverlap
  (params (OtherActor :type Actor%20Object%20Reference)))

(event EventTick
  (params (DeltaSeconds :type Float%20%28single-precision%29)))

(fn ConstructionScript)