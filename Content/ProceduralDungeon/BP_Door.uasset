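; Procedural dungeon door that the player opens with E to spawn the next room.
; While Ready, its DoorInteraction overlap shows an interact prompt and enables input for the player.
; Pressing E passes its exit and itself to BP_DungeonGenerator, calls SpawnNextRoom, then raises the door.
; Open and close timelines add per-update Z offsets, so travel depends on frame rate, and end in Opened or Closed state.
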(event OnComponentBeginOverlap(DoorInteraction)
  (params (OverlappedComponent :type Primitive%20Component%20Object%20Reference) (OtherActor :type Actor%20Object%20Reference) (OtherComp :type Primitive%20Component%20Object%20Reference) (OtherBodyIndex :type Integer) (bFromSweep :type Boolean) (SweepResult :type Hit%20Result%20Structure%20%28by%20ref%29))
  ;[0.03112 0.3897 1] Interaction with prompt
  (if (== OtherActor (Game|GetPlayerCharacter 0))
    (switch Utilities|FlowControl|Switch|SwitchonE_DoorState (Variables|Default|GetState)
      (:NewEnumerator0
        (UserInterface|Viewport|AddtoViewport (Variables|Default|GetInteract%20Prompt) 0)
        (Input|EnableInput (Game|GetPlayerController 0))))))

(event OnComponentEndOverlap(DoorInteraction)
  (params (OverlappedComponent :type Primitive%20Component%20Object%20Reference) (OtherActor :type Actor%20Object%20Reference) (OtherComp :type Primitive%20Component%20Object%20Reference) (OtherBodyIndex :type Integer))
  ;[0.03112 0.3897 1] Interaction with prompt
  (if (== (Game|GetPlayerCharacter 0) OtherActor)
    (switch Utilities|FlowControl|Switch|SwitchonE_DoorState (Variables|Default|GetState)
      (:NewEnumerator0
        (Widget|RemovefromParent (Variables|Default|GetInteract%20Prompt))
        (Input|DisableInput (Game|GetPlayerController 0))))))

(event Custom|Close%20Door
  (bind _door (Variables|Default|GetDoor))
  ;[0.5321 0.2538 1] Door closing animation
  (bind _doorfloat (Timeline|Шкала%20времени Play)
    (:Update
      (Transformation|SetRelativeLocation _door (- (Variables|/Script/Engine.SceneComponent|GetRelativeLocation _door) (Math|Vector|MakeVector 0.0 0.0 (Math|Float|Lerp 0.0 5.0 _doorfloat))) false false))
    (:Finished
      (Variables|Default|SetState "NewEnumerator4"))))

(event Custom|Open%20Door
  (bind _door (Variables|Default|GetDoor))
  ;[0.5321 0.2538 1] Door opening animation
  (bind _doorfloat (Timeline|Open%20Door%20Timeline PlayFromStart)
    (:Update
      (Transformation|SetRelativeLocation _door (+ (Variables|/Script/Engine.SceneComponent|GetRelativeLocation _door) (Math|Vector|MakeVector 0.0 0.0 (Math|Float|Lerp 0.0 5.0 _doorfloat))) false false))
    (:Finished
      (Variables|Default|SetState "NewEnumerator2"))))

(event EventBeginPlay
  ;[0.2206 0.8599 1] Defining prompt
  (bind _returnvalue (Game|ConstructObjectfromClass "/Game/BP_InteractPrompt.BP_InteractPrompt_C"))
  (Variables|Default|SetInteract%20Prompt _returnvalue))

(event Collision|EventActorBeginOverlap
  (params (OtherActor :type Actor%20Object%20Reference)))

(event EventTick
  (params (DeltaSeconds :type Float%20%28single-precision%29)))

(event Input|KeyboardEvents|E
  (params (Key :type Key%20Structure :default "None"))
  ;[0 0.03031 1] E button
  (:Pressed
    (Variables|Default|SetState "NewEnumerator1")
    (Widget|RemovefromParent (Variables|Default|GetInteract%20Prompt))
    (Input|DisableInput (Game|GetPlayerController 0))
    (bind _outactors (Actor|GetAllActorsOfClass "/Game/ProceduralDungeon/BP_DungeonGenerator.BP_DungeonGenerator_C"))
    (Variables|/Game/ProceduralDungeon/BP_DungeonGenerator.BP_DungeonGenerator_C|SetSelectedExit (Utilities|Array|Get(acopy) _outactors) (Variables|Default|GetExitReference))
    (Variables|/Game/ProceduralDungeon/BP_DungeonGenerator.BP_DungeonGenerator_C|SetSelectedDoor (Utilities|Array|Get(acopy) _outactors) self)
    (Default|SpawnNextRoom (Utilities|Array|Get(acopy) _outactors))
    (CallFunction|OpenDoor)))

(fn ConstructionScript)