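; BP_Projectile is a projectile in the procedural dungeon folder that damages and knocks back the player character on contact.
; A sphere overlap with the player launches BP_ThirdPersonCharacter using the projectile's velocity plus an upward boost, applies fixed damage and destroys the projectile.
; An overlap with any other actor destroys the projectile after a short delay.
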(event OnComponentBeginOverlap(Sphere)
  (params (OverlappedComponent :type Primitive%20Component%20Object%20Reference) (OtherActor :type Actor%20Object%20Reference) (OtherComp :type Primitive%20Component%20Object%20Reference) (OtherBodyIndex :type Integer) (bFromSweep :type Boolean) (SweepResult :type Hit%20Result%20Structure%20%28by%20ref%29))
  (bind _returnvalue (Game|GetPlayerCharacter 0))
  (if (== OtherActor _returnvalue)
    (bind _asbp_third_person_character (Utilities|Casting|CastToBP_ThirdPersonCharacter _returnvalue))
    (Character|LaunchCharacter _asbp_third_person_character (+ (Transformation|GetVelocity) "0.000000,0.000000,200.000000") false false)
    (Game|Damage|ApplyDamage _asbp_third_person_character 15.0 0 0)
    (Actor|DestroyActor)
    (else
      (Utilities|FlowControl|Delay 1.9)
      (Actor|DestroyActor))))

(fn ConstructionScript)