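; BP_MasterRoom is a procedural dungeon room that updates the generator's door and room state when its OverlapBox is entered.
; On any overlap, it finds the first BP_DungeonGenerator and branches on its SelectedDoor state.
; An open door is closed unless this room is the generator's LastRoom.
; A closed door instead causes LastRoom to be destroyed, with no check on the overlapping actor.
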(event OnComponentBeginOverlap(OverlapBox)
  (params (OverlappedComponent :type Primitive%20Component%20Object%20Reference) (OtherActor :type Actor%20Object%20Reference) (OtherComp :type Primitive%20Component%20Object%20Reference) (OtherBodyIndex :type Integer) (bFromSweep :type Boolean) (SweepResult :type Hit%20Result%20Structure%20%28by%20ref%29))
  (bind _outactors (Actor|GetAllActorsOfClass "/Game/ProceduralDungeon/BP_DungeonGenerator.BP_DungeonGenerator_C"))
  (switch Utilities|FlowControl|Switch|SwitchonE_DoorState (Variables|/Game/ProceduralDungeon/BP_Door.BP_Door_C|GetState (Variables|/Game/ProceduralDungeon/BP_DungeonGenerator.BP_DungeonGenerator_C|GetSelectedDoor (Utilities|Array|Get(acopy) _outactors)))
    (:NewEnumerator2
      (if (!= self (Variables|/Game/ProceduralDungeon/BP_DungeonGenerator.BP_DungeonGenerator_C|GetLastRoom (Utilities|Array|Get(acopy) _outactors)))
        (Default|CloseDoor (Variables|/Game/ProceduralDungeon/BP_DungeonGenerator.BP_DungeonGenerator_C|GetSelectedDoor (Utilities|Array|Get(acopy) _outactors)))))
    (:NewEnumerator4
      (Actor|DestroyActor (Variables|/Game/ProceduralDungeon/BP_DungeonGenerator.BP_DungeonGenerator_C|GetLastRoom (Utilities|Array|Get(acopy) _outactors))))))

(event EventBeginPlay)

(event Collision|EventActorBeginOverlap
  (params (OtherActor :type Actor%20Object%20Reference)))

(event EventTick
  (params (DeltaSeconds :type Float%20%28single-precision%29)))

(fn ConstructionScript)