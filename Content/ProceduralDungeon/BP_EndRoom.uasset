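; End room actor for the procedural dungeon, where the player claims the prize to win.
; An interact prompt is built on BeginPlay and shown while the player character overlaps PrizeInteraction, which also toggles the actor's input.
; Pressing E swaps the prompt for a win widget, shows the mouse cursor and switches to UI-only input.
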(event OnComponentBeginOverlap(PrizeInteraction)
  (params (OverlappedComponent :type Primitive%20Component%20Object%20Reference) (OtherActor :type Actor%20Object%20Reference) (OtherComp :type Primitive%20Component%20Object%20Reference) (OtherBodyIndex :type Integer) (bFromSweep :type Boolean) (SweepResult :type Hit%20Result%20Structure%20%28by%20ref%29))
  ;[0.03112 0.3897 1] Interaction with prompt
  (if (== OtherActor (Game|GetPlayerCharacter 0))
    (UserInterface|Viewport|AddtoViewport (Variables|Default|GetInteract%20Prompt) 0)
    (Input|EnableInput (Game|GetPlayerController 0))))

(event OnComponentEndOverlap(PrizeInteraction)
  (params (OverlappedComponent :type Primitive%20Component%20Object%20Reference) (OtherActor :type Actor%20Object%20Reference) (OtherComp :type Primitive%20Component%20Object%20Reference) (OtherBodyIndex :type Integer))
  ;[0.03112 0.3897 1] Interaction with prompt
  (if (== (Game|GetPlayerCharacter 0) OtherActor)
    (Widget|RemovefromParent (Variables|Default|GetInteract%20Prompt))
    (Input|DisableInput (Game|GetPlayerController 0))))

(event EventBeginPlay
  ;[0.1418 1 0] Setup
  (|CallParentFunction)
  (bind _returnvalue (Game|ConstructObjectfromClass "/Game/BP_InteractPrompt.BP_InteractPrompt_C"))
  (Variables|Default|SetInteract%20Prompt _returnvalue))

(event Collision|EventActorBeginOverlap
  (params (OtherActor :type Actor%20Object%20Reference))
  (|CallParentFunction OtherActor) ; Этот узел отключен и не будет вызываться.\nПеретащите контакты, чтобы построить функционал.
)

(event EventTick
  (params (DeltaSeconds :type Float%20%28single-precision%29))
  (|CallParentFunction DeltaSeconds) ; Этот узел отключен и не будет вызываться.\nПеретащите контакты, чтобы построить функционал.
)

(event Input|KeyboardEvents|E
  (params (Key :type Key%20Structure :default "None"))
  (bind _returnvalue (Game|GetPlayerController 0))
  ;[1 0.9626 0] Press E to win
  (:Pressed
    (Widget|RemovefromParent (Variables|Default|GetInteract%20Prompt))
    (bind _returnvalue_2 (UserInterface|CreateWidget "/Game/BP_WinPrompt.BP_WinPrompt_C"))
    (UserInterface|Viewport|AddtoViewport _returnvalue_2 0)
    (Variables|/Script/Engine.PlayerController|SetbShowMouseCursor _returnvalue true)
    (Input|SetInputModeUIOnly _returnvalue 0 "DoNotLock" false)))

(fn ConstructionScript
  (|CallParentFunction))